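; bp_matHit is an actor that turns blue and shrinks each time another actor overlaps it.
; BeginPlay stores five percent of StartScale as a fixed DeltaScale step.
; Each overlap sets Cube0's material to AnimSharingBlue, subtracts that step from StartScale and applies the result as actor scale, so shrinking is linear with no lower limit.
; Tick is disabled and the construction script only calls its parent.
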(event `self.ReceiveBeginPlay`
  (`parent.ReceiveBeginPlay`)
  (bind _output_get (set `self.delta_scale` (* (`self.start_scale`) (0.05 0.05 0.05)))))

(event `self.ReceiveActorBeginOverlap`
  (params (OtherActor :type "Actor Object Reference"))
  (`parent.ReceiveActorBeginOverlap` OtherActor)
  (`PrimitiveComponent.SetMaterial` (`self.Cube_0`) 0 "/AnimationSharing/AnimSharingBlue.AnimSharingBlue")
  (bind _output_get (set `self.start_scale` (- (`self.start_scale`) (stale `self.ReceiveBeginPlay` _output_get))))
  (`self.SetActorScale3D` _output_get))

(fn `UserConstructionScript`
  (`parent.UserConstructionScript`))