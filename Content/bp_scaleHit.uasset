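; Actor Blueprint that shrinks itself each time another actor begins overlapping it.
; BeginPlay stores five percent of the starting scale as a fixed step and immediately applies one shrink.
; Each overlap jumps into that same chain, subtracting the step linearly with no lower limit, setting the actor's scale and printing it for debugging.
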(event `self.ReceiveBeginPlay`
  (`parent.ReceiveBeginPlay`)
  (bind _output_get (set `self.delta_scale` (* (`self.start_scale`) (0.05 0.05 0.05))))
  (bind _output_get_2 (set `self.start_scale` (- (`self.start_scale`) _output_get) :!label _label))
  (`self.SetActorScale3D` _output_get_2)
  (`KismetSystemLibrary.PrintString` (`KismetStringLibrary.Conv_VectorToString` _output_get_2) true true (struct :`G` 0.66 :`B` 1.0 :`A` 1.0) 10.0))

(event `self.ReceiveActorBeginOverlap`
  (params (OtherActor :type "Actor Object Reference"))
  (`parent.ReceiveActorBeginOverlap` OtherActor)
  (goto _label))

(event `self.ReceiveTick`
  (params (DeltaSeconds :type "Float (single-precision)"))
  (`parent.ReceiveTick` DeltaSeconds))

(fn `UserConstructionScript`
  (`parent.UserConstructionScript`))